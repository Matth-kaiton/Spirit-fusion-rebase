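; BP_enemie is an enemy Blueprint that displays its health on a HealBar widget component.
; Every Tick it casts the widget to Health_bar and sets the progress bar from CurrentHealth, assuming a maximum of 100.
; It then rotates the bar toward player 0's camera, billboard style, and the update stops if the cast fails.
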(event `self.ReceiveTick`
  (params (DeltaSeconds :type "Float (single-precision)"))
  (bind _heal_bar (`self.heal_bar`))
  (bind _ashealth_bar (cast `/Game/Spirit_fusion/Blueprint/Health_bar` (`WidgetComponent.GetWidget` (`self.heal_bar`))))
  (`ProgressBar.SetPercent` (`/Game/Spirit_fusion/Blueprint/Health_bar.ProgressBar_0` _ashealth_bar) (/ (`self.CurrentHealth`) 100.0))
  (`SceneComponent.K2_SetWorldRotation` _heal_bar (`KismetMathLibrary.FindLookAtRotation` (`SceneComponent.K2_GetComponentLocation` _heal_bar) (`SceneComponent.K2_GetComponentLocation` (`PlayerCameraManager.TransformComponent` (`GameplayStatics.GetPlayerCameraManager` 0)))) false false))

(fn `UserConstructionScript`)