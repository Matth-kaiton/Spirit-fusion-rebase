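; Fireball actor in the tower folder that deals short-lived area damage to enemies.
; Tick runs through a latent 0.2-second Delay, so the damage event repeats at roughly that interval until a second Delay destroys the actor after about three seconds.
; Each pulse subtracts fixed damage directly from the CurrentHealth of every BP_enemie overlapping its Sphere.
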(event `self.ReceiveTick`
  (params (DeltaSeconds :type "Float (single-precision)"))
  (`KismetSystemLibrary.Delay` 0.2)
  (`self.damageDeal`)
  (`KismetSystemLibrary.Delay` 3.0)
  (`self.K2_DestroyActor`))

(event `damageDeal`
  (for _array_element (`PrimitiveComponent.GetOverlappingActors` (`self.Sphere`) "/Game/Spirit_fusion/Blueprint/Enemie/BP_enemie.BP_enemie_C")
    (bind _asbp_enemie (cast `/Game/Spirit_fusion/Blueprint/Enemie/BP_enemie` _array_element))
    (set `/Game/Spirit_fusion/Blueprint/Enemie/BP_enemie.CurrentHealth` (- (`/Game/Spirit_fusion/Blueprint/Enemie/BP_enemie.CurrentHealth` _asbp_enemie) 5.0) _asbp_enemie)))

(fn `UserConstructionScript`)