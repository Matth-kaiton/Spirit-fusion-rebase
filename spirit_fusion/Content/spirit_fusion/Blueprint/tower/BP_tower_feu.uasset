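; Fire tower Blueprint for a tower defense setup that attacks BP_enemie actors inside its overlap area.
; Begin and end overlap events maintain the enemy list, and a new target is the nearest actor in that list.
; The self-calling Hitter event subtracts health directly, spawns a fireball at the target, destroys it at zero health, then repeats after a cooldown delay.
; The BurnZone function is an empty stub.
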(event `self.ReceiveActorBeginOverlap`
  (params (OtherActor :type "Actor Object Reference"))
  (if (`KismetMathLibrary.ClassIsChildOf` (`GameplayStatics.GetObjectClass` OtherActor) "/Game/Spirit_fusion/Blueprint/Enemie/BP_enemie.BP_enemie_C")
    (`KismetArrayLibrary.Array_Add` (`self.AllEnemy`) OtherActor)
    (`self.Hitter`)))

(event `self.ReceiveActorEndOverlap`
  (params (OtherActor :type "Actor Object Reference"))
  (if (== OtherActor (`self.target`))
    (set `self.in_range` false))
  (`KismetArrayLibrary.Array_RemoveItem` (`self.AllEnemy`) OtherActor))

(event `Hitter`
  (if (`self.new target`)
    (`self.set Target`))
  (if (`self.cooldown`)
    (set `self.cooldown` false)
    (if (`self.in_range`)
      (bind _asbp_enemie (cast `/Game/Spirit_fusion/Blueprint/Enemie/BP_enemie` (`self.target`)))
      (set `/Game/Spirit_fusion/Blueprint/Enemie/BP_enemie.CurrentHealth` (- (`/Game/Spirit_fusion/Blueprint/Enemie/BP_enemie.CurrentHealth` _asbp_enemie) (`self.attPower`)) _asbp_enemie)
      (`|SpawnActorFromClass` "/Game/Spirit_fusion/Blueprint/tower/firebal.firebal_C" (`KismetMathLibrary.Conv_VectorToTransform` (`self.K2_GetActorLocation` _asbp_enemie)) "Undefined" "MultiplyWithRoot" null null)
      (if (not (> (`/Game/Spirit_fusion/Blueprint/Enemie/BP_enemie.CurrentHealth` _asbp_enemie) 0.0))
        (`self.K2_DestroyActor` _asbp_enemie)
        (set `self.in_range` false)
        (set `self.new target` true))
      (if (not (`KismetArrayLibrary.Array_IsEmpty` (`self.AllEnemy`)))
        (`KismetSystemLibrary.Delay` (`self.attCooldown`))
        (set `self.cooldown` true)
        (`self.Hitter`))
      (else
        (set `self.new target` true)
        (`self.Hitter`)))))

(event `set Target`
  (set `self.new target` false)
  (set `self.target` (`.ReturnValue` (`GameplayStatics.FindNearestActor` (`self.K2_GetActorLocation`) (`self.AllEnemy`))))
  (set `self.in_range` true))

(fn `Burn Zone`
  (params (`Ennemi position` :type "Vector Structure")))

(fn `UserConstructionScript`)